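; Player Blueprint for Rockube that prototypes rhythm timing feedback alongside a dash.
; BeginPlay creates HUD widgets and subscribes to Beat quantization on the BeatSync counter's Quartz clock, pulsing a BPM hint each beat.
; P starts the clock, while N is a temporary hit test that grades timing as Perfect, Good or Miss via widgets and debug prints.
; Left Shift forwards dash input to RockubeMovmentComponent, independent of the beat check.
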(event Custom|OnBeat)

(event Custom|Clock%20Event
  (params (ClockName :type Name) (QuantizationType :type EQuartzCommandQuantization%20Enum :default "Bar") (NumBars :type Integer) (Beat :type Integer) (BeatFraction :type Float%20%28single-precision%29))
  (switch Utilities|FlowControl|Switch|SwitchonEQuartzCommandQuantization QuantizationType
    (:Beat
      (Default|UpdateOpacity (Variables|Default|GetHUD_BPMHint)))))

(event EventBeginPlay
  (bind _returnvalue (UserInterface|CreateWidget "/Game/HUD/WBP_BPMHInt.WBP_BPMHInt_C"))
  (bind _output_get (Variables|Default|SetHUD_BPMHint _returnvalue))
  (UserInterface|Viewport|AddtoViewport _output_get 0)
  (bind _returnvalue_2 (Class|BeatSyncComponent|GetBPMCounter (Variables|Default|GetBeatSync)))
  (bind _output_get_2 (Variables|Default|SetGlobalBPMTickRef _returnvalue_2))
  (bind _returnvalue_3 (Class|QuartzSubsystem|GetHandleforClock (WorldSubsystems|GetQuartzSubsystem) (Variables|/Script/Rockube.GlobalBPMTickCounter|GetQuartzClockName (Variables|Default|GetGlobalBPMTickRef))))
  (bind _output_get_3 (Variables|Default|SetClockHandle _returnvalue_3))
  (Class|QuartzClockHandle|SubscribetoQuantizationEvent _output_get_3 "Beat" (delegate Custom|Clock%20Event))
  (bind _returnvalue_4 (UserInterface|CreateWidget "/Game/HUD/WBP_Perfect.WBP_Perfect_C"))
  (bind _output_get_4 (Variables|Default|SetHUD_Perfect _returnvalue_4))
  (UserInterface|Viewport|AddtoViewport _output_get_4 0)
  (bind _returnvalue_5 (UserInterface|CreateWidget "/Game/HUD/WBP_Good.WBP_Good_C"))
  (bind _output_get_5 (Variables|Default|SetHUD_Good _returnvalue_5))
  (UserInterface|Viewport|AddtoViewport _output_get_5 0)
  (bind _returnvalue_6 (UserInterface|CreateWidget "/Game/HUD/WBP_Miss.WBP_Miss_C"))
  (bind _output_get_6 (Variables|Default|SetHUD_Miss _returnvalue_6))
  (UserInterface|Viewport|AddtoViewport _output_get_6 0)
  (Variables|Default|SetbAllowedToPlay true))

(event Input|KeyboardEvents|N
  (params (Key :type Key%20Structure :default "None"))
  ;[1 1 1] Temporal On Beat Hit Checker
  (:Pressed
    (bind (_bisperfect _deltaerror _returnvalue) (Class|GlobalBPMTickCounter|IsonBeat (Variables|Default|GetGlobalBPMTickRef) 0.1 0.05))
    (bind _output_get (Variables|Default|SetDeltaError _deltaerror))
    (if _returnvalue
      (if _bisperfect
        (Development|PrintString (Utilities|String|Append (Utilities|String|MakeLiteralString "Perfect! Delta error: ") (Utilities|String|ToString(Float) _output_get)) true false "(R=0.000000,G=1.000000,B=0.301661,A=1.000000)" 1.0)
        (Default|UpdateOpacity (Variables|Default|GetHUD_Perfect))
        (else
          (Development|PrintString (Utilities|String|Append (Utilities|String|MakeLiteralString "Good. Delta error: ") (Utilities|String|ToString(Float) _output_get)) true false "(R=1.000000,G=0.796708,B=0.000000,A=1.000000)" 1.0)
          (Default|UpdateOpacity (Variables|Default|GetHUD_Good))))
      (else
        (Development|PrintString (Utilities|String|Append (Utilities|String|MakeLiteralString "Miss. Delta error: ") (Utilities|String|ToString(Float) _output_get)) true false "(R=1.000000,G=0.056476,B=0.000000,A=1.000000)" 1.0)
        (Default|UpdateOpacity (Variables|Default|GetHUD_Miss))))))

(event Input|KeyboardEvents|P
  (params (Key :type Key%20Structure :default "None"))
  (:Pressed
    (if (Variables|Default|GetbAllowedToPlay)
      (Class|QuartzClockHandle|StartClock (Variables|Default|GetClockHandle)))))

(event Input|KeyboardEvents|LeftShift
  (params (Key :type Key%20Structure :default "None"))
  (bind _rockubemovmentcomponent (Variables|Default|GetRockubeMovmentComponent))
  (:Pressed
    (Class|RockubeMovementComponent|DashPressed _rockubemovmentcomponent)
    (Development|PrintString "Dash" true true "(R=0.000000,G=1.000000,B=0.250000,A=1.000000)"))
  (:Released
    (Class|RockubeMovementComponent|DashReleased _rockubemovmentcomponent)))

(fn ConstructionScript)