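; Global BPM tick counter that creates a Quartz clock in 4/4 at a configurable BPM to provide a beat pulse.
; On BeginPlay it creates the named clock, sets its tempo and subscribes to all quantization events; no start call appears here.
; ClockEvent filters those events to Beat, calling PerformQuartzBeat and printing the bar and beat for debugging.
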(event Custom|ClockEvent
  (params (ClockName :type Name) (QuantizationType :type EQuartzCommandQuantization%20Enum :default "Bar") (NumBars :type Integer) (Beat :type Integer) (BeatFraction :type Float%20%28single-precision%29))
  (switch Utilities|FlowControl|Switch|SwitchonEQuartzCommandQuantization QuantizationType
    (:Beat
      (Class|GlobalBPMTickCounter|PerformQuartzBeat)
      (Development|PrintText (Utilities|Text|FormatText "Bar: {bar}   Beat: {beat}" NumBars Beat) true true "(R=0.924674,G=0.462254,B=1.000000,A=1.000000)"))))

(event EventBeginPlay
  (bind _returnvalue (Class|QuartzSubsystem|CreateNewClock (WorldSubsystems|GetQuartzSubsystem) (Variables|Default|GetQuartzClockName) (Utilities|Struct|MakeQuartzClockSettings (Utilities|Struct|MakeQuartzTimeSignature 4 "QuarterNote") false) false))
  (Development|PrintString "Clock created" true true "(R=1.000000,G=0.000000,B=0.722723,A=1.000000)")
  (bind _output_get (Variables|Default|SetQuartzClock _returnvalue))
  (bind _clockhandle (Class|QuartzClockHandle|SetBeatsPerMinute :self _output_get :BeatsPerMinute (Variables|Default|GetBPM)))
  (Class|QuartzClockHandle|SubscribetoAllQuantizationEvents _clockhandle (delegate Custom|ClockEvent)))

(fn ConstructionScript)