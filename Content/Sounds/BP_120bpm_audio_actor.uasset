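; Audio actor, named for 120 bpm, that plays its sound in time with a shared Quartz clock and starts the game's beat counter.
; After a short delay on BeginPlay, it gets the BPM counter from BeatSync, resolves that counter's clock and queues playback quantized to the beat.
; When playback reports Started, it calls StartBeatTick on the counter.
; An alternate clock lookup and quantization subscription are left unconnected.
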(event Custom|PlayStarted
  (params (EventType :type EQuartzCommandDelegateSubType%20Enum :default "CommandOnFailedToQueue") (Name :type Name))
  (switch Utilities|FlowControl|Switch|SwitchonEQuartzCommandDelegateSubType EventType
    (:CommandOnQueued
      (Development|PrintString "Qued"))
    (:CommandOnStarted
      (Development|PrintString "started")
      (Class|GlobalBPMTickCounter|StartBeatTick (Variables|Default|GetBPMCounterRef)))))

(event Custom|Clock%20Event
  (params (ClockName :type Name) (QuantizationType :type EQuartzCommandQuantization%20Enum :default "Bar") (NumBars :type Integer) (Beat :type Integer) (BeatFraction :type Float%20%28single-precision%29)))

(event EventBeginPlay
  (Utilities|FlowControl|Delay 0.2)
  (Development|PrintString "Acessing counter")
  (bind _returnvalue (Class|BeatSyncComponent|GetBPMCounter (Variables|Default|GetBeatSync)))
  (bind _output_get (Variables|Default|SetBPMCounterRef _returnvalue))
  (bind _returnvalue_2 (Class|QuartzSubsystem|GetHandleforClock (WorldSubsystems|GetQuartzSubsystem) (Variables|/Script/Rockube.GlobalBPMTickCounter|GetQuartzClockName _output_get)))
  (bind _output_get_2 (Variables|Default|SetGlobalClockRef _returnvalue_2))
  (Audio|Components|Audio|PlayQuantized (Variables|Default|GetAudio) _output_get_2 (Utilities|Struct|MakeQuartzQuantizationBoundary "Beat" 1.0 "BarRelative") (delegate Custom|PlayStarted)))

(fn ConstructionScript)